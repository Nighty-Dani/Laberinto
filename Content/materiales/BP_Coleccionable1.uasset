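; BP_Coleccionable1 is a wandering collectible pawn that roams the terrain and is picked up by the player.
; Tick runs a five-second Delay, then sends the pawn via AIMoveTo to a random reachable navmesh point within a radius of its location.
; When a BP_ThirdPersonCharacter overlaps its Box, it adds score through Sumarpuntaje, calls CollectItem on the BP_puerta door found by class, and destroys itself.
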(event OnComponentBeginOverlap(Box)
  (params (OverlappedComponent :type Primitive%20Component%20Object%20Reference) (OtherActor :type Actor%20Object%20Reference) (OtherComp :type Primitive%20Component%20Object%20Reference) (OtherBodyIndex :type Integer) (bFromSweep :type Boolean) (SweepResult :type Hit%20Result%20Structure%20%28by%20ref%29))
  (bind _asbp_third_person_character (Utilities|Casting|CastToBP_ThirdPersonCharacter OtherActor))
  (Default|Sumarpuntaje _asbp_third_person_character)
  (bind _returnvalue (Actor|GetActorOfClass "/Game/materiales/BP_puerta.BP_puerta_C"))
  (Default|CollectItem _returnvalue)
  (Actor|DestroyActor))

(event EventTick
  (params (DeltaSeconds :type Float%20%28single-precision%29))
  ;[0.05098 0.05098 0.05098] Pratullamiento del Terreno
  (Utilities|FlowControl|Delay 5.0)
  (AI|AIMoveTo self (.RandomLocation (AI|Navigation|GetRandomReachablePointinRadius (Transformation|GetActorLocation) 2e+03 0 0)) 0 5.0 false))

(fn ConstructionScript)