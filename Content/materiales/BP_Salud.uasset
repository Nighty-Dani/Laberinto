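; BP_Salud is a health pickup actor triggered when BP_ThirdPersonCharacter overlaps its Box component.
; On overlap it stores the character and sets a Detection flag, then compares the character's VidaAct to VidaTot.
; If health is below the total, it adds a fixed amount without clamping and destroys itself after a short delay.
; At full health the pickup stays in place.
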(event OnComponentBeginOverlap(Box)
  (params (OverlappedComponent :type Primitive%20Component%20Object%20Reference) (OtherActor :type Actor%20Object%20Reference) (OtherComp :type Primitive%20Component%20Object%20Reference) (OtherBodyIndex :type Integer) (bFromSweep :type Boolean) (SweepResult :type Hit%20Result%20Structure%20%28by%20ref%29))
  (bind _asbp_third_person_character (Utilities|Casting|CastToBP_ThirdPersonCharacter OtherActor))
  (Variables|Default|SetAs%20BP%20Third%20Person%20Character _asbp_third_person_character)
  (Variables|Default|SetDetection true)
  (if (and (< (Variables|/Game/ThirdPerson/Blueprints/BP_ThirdPersonCharacter.BP_ThirdPersonCharacter_C|Getvida%20Act (Variables|Default|GetAs%20BP%20Third%20Person%20Character)) (Variables|/Game/ThirdPerson/Blueprints/BP_ThirdPersonCharacter.BP_ThirdPersonCharacter_C|Getvida%20Tot (Variables|Default|GetAs%20BP%20Third%20Person%20Character))) (Variables|Default|GetDetection))
    (Variables|/Game/ThirdPerson/Blueprints/BP_ThirdPersonCharacter.BP_ThirdPersonCharacter_C|Setvida%20Act (Variables|Default|GetAs%20BP%20Third%20Person%20Character) (+ (Variables|/Game/ThirdPerson/Blueprints/BP_ThirdPersonCharacter.BP_ThirdPersonCharacter_C|Getvida%20Act (Variables|Default|GetAs%20BP%20Third%20Person%20Character)) 1e+02))
    (Utilities|FlowControl|Delay 0.2)
    (Actor|DestroyActor)))

(event EventBeginPlay)

(event Collision|EventActorBeginOverlap
  (params (OtherActor :type Actor%20Object%20Reference)))

(event EventTick
  (params (DeltaSeconds :type Float%20%28single-precision%29)))

(fn ConstructionScript)