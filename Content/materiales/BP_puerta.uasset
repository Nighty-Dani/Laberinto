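; Door Blueprint that swings open once enough items have been collected.
; Collectitem increments the collected count, and OpenDoorCheck compares it to the maximum, using a DoOnce to trigger the opening a single time.
; Opendoor plays a timeline whose DoorRotation track lerps the door component's relative yaw from closed to open.
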(event Custom|Open%20door
  (bind _door_rotation (Timeline|Open%20door%20anim Play)
    (:Update
      (Transformation|SetRelativeRotation (Variables|Default|GetPuerta) (Math|Rotator|MakeRotator 0.0 0.0 (Math|Float|Lerp 0.0 1.2e+02 _door_rotation)) false false))))

(event Custom|Collect%20item
  (Math|Integer|IncrementInt (Variables|Default|GetcurrentItemsCollected)))

(event Custom|Open%20Door%20Check
  (if (>= (Variables|Default|GetcurrentItemsCollected) (Variables|Default|GetmaxItemsCollectable))
    (Utilities|FlowControl|DoOnce false
      (:Completed
        (CallFunction|OpenDoor)))))

(fn ConstructionScript)