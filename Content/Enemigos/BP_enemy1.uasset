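; BP_enemy1 is an enemy that wanders randomly and chases the player by sound, with melee attack animations.
; Tick issues delayed moves to random reachable points until PawnSensing hears the player, then follows them at raised speed, slowing if the move fails.
; A retriggerable delay ends the chase shortly after the last noise.
; Box overlaps with the player toggle the Attack flag in the BPC_anim_huesos animation blueprint.
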(event OnHearNoise(PawnSensing)
  (params (Instigator :type Pawn%20Object%20Reference) (Location :type Vector%20%28by%20ref%29 :default "0, 0, 0") (Volume :type Float%20%28single-precision%29))
  (bind _charactermovement (Variables|Character|GetCharacterMovement))
  ;[0.05098 0.05098 0.05098] Seguimiento por Ruido
  (bind _asbp_third_person_character (Utilities|Casting|CastToBP_ThirdPersonCharacter Instigator))
  (Utilities|FlowControl|Sequence
    (:then_0
      (Variables|Default|Setpuede%20oirnos? true)
      (AI|AIMoveTo self Location _asbp_third_person_character 5.0 false
        (:then
          (Variables|/Script/Engine.CharacterMovementComponent|SetMaxWalkSpeed _charactermovement 6e+02))
        (:OnFail
          (Variables|/Script/Engine.CharacterMovementComponent|SetMaxWalkSpeed _charactermovement 3e+02))))
    (:then_1
      (Utilities|FlowControl|RetriggerableDelay 3.0)
      (Variables|Default|Setpuede%20oirnos? false))))

(event OnComponentBeginOverlap(Box)
  (params (OverlappedComponent :type Primitive%20Component%20Object%20Reference) (OtherActor :type Actor%20Object%20Reference) (OtherComp :type Primitive%20Component%20Object%20Reference) (OtherBodyIndex :type Integer) (bFromSweep :type Boolean) (SweepResult :type Hit%20Result%20Structure%20%28by%20ref%29))
  (Utilities|Casting|CastToBP_ThirdPersonCharacter OtherActor)
  (bind _asbpc_anim_huesos (Utilities|Casting|CastToBPC_anim_huesos (Components|SkeletalMesh|GetAnimInstance (Variables|Character|GetMesh))))
  (Variables|/Game/Enemigos/animation/BPC_anim_huesos.BPC_anim_huesos_C|Setattack? _asbpc_anim_huesos true))

(event OnComponentEndOverlap(Box)
  (params (OverlappedComponent :type Primitive%20Component%20Object%20Reference) (OtherActor :type Actor%20Object%20Reference) (OtherComp :type Primitive%20Component%20Object%20Reference) (OtherBodyIndex :type Integer))
  (Utilities|Casting|CastToBP_ThirdPersonCharacter OtherActor)
  (bind _asbpc_anim_huesos (Utilities|Casting|CastToBPC_anim_huesos (Components|SkeletalMesh|GetAnimInstance (Variables|Character|GetMesh))))
  (Variables|/Game/Enemigos/animation/BPC_anim_huesos.BPC_anim_huesos_C|Setattack? _asbpc_anim_huesos false))

(event EventTick
  (params (DeltaSeconds :type Float%20%28single-precision%29))
  (bind _charactermovement (Variables|Character|GetCharacterMovement))
  ;[0.05098 0.05098 0.05098] Pratullamiento del Terreno
  (if (Variables|Default|Getpuede%20oirnos?)
    ;[0.05098 0.05098 0.05098] Seguimiento por Ruido
    (AI|AIMoveTo self (stale OnHearNoise(PawnSensing) Location) (stale OnHearNoise(PawnSensing) _asbp_third_person_character) 5.0 false
      (:then
        (Variables|/Script/Engine.CharacterMovementComponent|SetMaxWalkSpeed _charactermovement 6e+02))
      (:OnFail
        (Variables|/Script/Engine.CharacterMovementComponent|SetMaxWalkSpeed _charactermovement 3e+02)))
    (else
      (Utilities|FlowControl|Delay 3.0)
      (AI|AIMoveTo self (.RandomLocation (AI|Navigation|GetRandomReachablePointinRadius (Transformation|GetActorLocation) 2e+03 0 0)) 0 5.0 false))))

(fn ConstructionScript)